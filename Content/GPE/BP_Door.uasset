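; BP_Door is a door actor that destroys itself once no BP_Target actors from its list remain.
; On BeginPlay it collects every BP_Target in the level into TargetList.
; Each Tick it prunes invalid entries from that list and calls DestroyActor when the list is empty, polling rather than binding to destruction events.
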(event EventBeginPlay
  (bind _outactors (Actor|GetAllActorsOfClass "/Game/GPE/BP_Target.BP_Target_C"))
  (Variables|Default|SetTargetList _outactors))

(event EventTick
  (params (DeltaSeconds :type Float%20%28single-precision%29))
  (bind _targetlist (Variables|Default|GetTargetList))
  (for _array_element _targetlist
    (Utilities|IsValid _array_element
      (:Is%20Not%20Valid
        (Utilities|Array|RemoveItem _targetlist _array_element))))
  (if (== (Utilities|Array|Length _targetlist) 0)
    (Actor|DestroyActor)))

(fn ConstructionScript)