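; BP_Holy is a spinning cube actor that reacts with divine wrath when hit.
; Each tick it rotates the cube on all three axes, scaled by a speed multiplier.
; A hit flags it as dead and prints a long-lasting red warning that the gods are angered.
; Once dead, the multiplier grows every frame, so the spin accelerates exponentially, tied to frame rate.
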(event EventBeginPlay)

(event Collision|EventActorBeginOverlap
  (params (OtherActor :type Actor%20Object%20Reference)))

(event EventTick
  (params (DeltaSeconds :type Float%20%28single-precision%29))
  (Transformation|AddWorldRotation (Variables|Default|GetCube) (Math|Rotator|MakeRotator (* 1.0 (Variables|Default|GetMultiplySpeed)) (* 1.2 (Variables|Default|GetMultiplySpeed)) (* 0.8 (Variables|Default|GetMultiplySpeed))) false false)
  (if (Variables|Default|GetisDead)
    (Variables|Default|SetMultiplySpeed (* (Variables|Default|GetMultiplySpeed) 1.02))))

(event Collision|EventHit
  (params (MyComp :type Primitive%20Component%20Object%20Reference) (Other :type Actor%20Object%20Reference) (OtherComp :type Primitive%20Component%20Object%20Reference) (bSelfMoved :type Boolean) (HitLocation :type Vector :default "0, 0, 0") (HitNormal :type Vector :default "0, 0, 0") (NormalImpulse :type Vector :default "0, 0, 0") (Hit :type Hit%20Result%20Structure%20%28by%20ref%29))
  (Variables|Default|SetisDead true)
  (Development|PrintString "You have angered the gods" true true "(R=0.692708,G=0.000000,B=0.019199,A=1.000000)" 1e+03))

(fn ConstructionScript)