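; Player character Blueprint that tracks movement speed and direction relative to the camera and offers walk/run switching.
; Tick derives a normalized SpeedRatio from velocity and a signed SpeedDir angle via atan2 of the 2D cross and dot products against camera forward, printing the angle on screen.
; While moving, the mesh snaps to camera yaw with an offset.
; The Run function toggles max walk speed between walking and running values.
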(event EventBeginPlay)

(event Collision|EventActorBeginOverlap
  (params (OtherActor :type Actor%20Object%20Reference)))

(event EventTick
  (params (DeltaSeconds :type Float%20%28single-precision%29))
  (bind _charactermovement (Variables|Character|GetCharacterMovement))
  (bind _camera (Variables|Default|GetCamera))
  (bind _returnvalue (Math|Vector|GetForwardVector _camera))
  (bind _velocity (Variables|/Script/Engine.MovementComponent|GetVelocity _charactermovement))
  (bind _returnvalue_2 (Math|Vector2D|MakeVector2D (.x _velocity) (.y _velocity)))
  (bind _returnvalue_3 (Math|Vector2D|MakeVector2D (.x _returnvalue) (.y _returnvalue)))
  (bind _returnvalue_4 (Math|Vector2D|Normalize2D _returnvalue_2))
  (bind _returnvalue_5 (Math|Vector2D|Normalize2D _returnvalue_3))
  (bind (_x _y) (Math|Vector2D|BreakVector2D _returnvalue_4))
  (bind (_x_2 _y_2) (Math|Vector2D|BreakVector2D _returnvalue_5))
  (Variables|Default|SetSpeedRatio (Math|Float|MapRangeClamped (Math|Vector|VectorLength (Variables|/Script/Engine.MovementComponent|GetVelocity (Variables|Character|GetCharacterMovement))) 0.0 1e+03 0.0 1.0))
  (bind _output_get (Variables|Default|SetSpeedDir (Class|KismetMathLibrary|DegAtan2 (- (* _x _y_2) (* _x_2 _y)) (Math|Vector2D|DotProduct(2D) _returnvalue_4 _returnvalue_5))))
  (Development|PrintString (Utilities|String|ToString(Float) _output_get))
  (if (not (Math|Vector|VectorIsNearlyZero (Variables|/Script/Engine.MovementComponent|GetVelocity _charactermovement)))
    (Transformation|SetWorldRotation (Variables|Character|GetMesh) (Math|Rotator|MakeRotator 0.0 0.0 (+ (.yaw (Transformation|GetWorldRotation (Variables|Default|GetCamera))) -9e+01)) false false)))

(fn ConstructionScript)

(fn Run
  (params (isRunning :type Boolean))
  (bind _charactermovement (Variables|Character|GetCharacterMovement))
  (if isRunning
    (Variables|/Script/Engine.CharacterMovementComponent|SetMaxWalkSpeed _charactermovement 1e+03)
    (else
      (Variables|/Script/Engine.CharacterMovementComponent|SetMaxWalkSpeed _charactermovement 4e+02))))