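; Player controller that maps Enhanced Input to third-person look, movement and sprint on BP_PlayerCharacter.
; BeginPlay adds IMC_Main, caches the character and seeds camera rotation from its BoomStick.
; Look input sets the boom's world rotation directly with clamped pitch, and movement follows the camera's flattened forward and right vectors.
; Sprint toggles when its input completes or cancels, and ending movement resets it, with both passed to the character's Run.
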(event Input|EnhancedActionEvents|EnhancedInputActionIA_Move
  (params (ActionValue :type Vector%202D%20Structure) (ElapsedSeconds :type Float%20%28double-precision%29) (TriggeredSeconds :type Float%20%28double-precision%29) (InputAction :type Input%20Action%20Object%20Reference :default "/Game/_GameManager/Inputs/InputActions/IA_Move.IA_Move"))
  (bind (_x _y) (Math|Vector2D|BreakVector2D ActionValue))
  (bind _playerchar (Variables|Default|GetPlayerChar))
  (bind _camera (Variables|/Game/_GameManager/BP_PlayerCharacter.BP_PlayerCharacter_C|GetCamera _playerchar))
  (bind _returnvalue (Math|Vector|GetForwardVector _camera))
  (bind _returnvalue_2 (Math|Vector|GetRightVector _camera))
  ;[1 1 1] Movement
  (:Triggered
    (Pawn|Input|AddMovementInput _playerchar (+ (* (Math|Vector|Normalize (Math|Vector|MakeVector (.x _returnvalue) (.y _returnvalue) 0.0)) _y) (* (Math|Vector|Normalize (Math|Vector|MakeVector (.x _returnvalue_2) (.y _returnvalue_2) 0.0)) _x)) 1.0 false))
  (:Canceled
    (bind _output_get (Variables|Default|SetisRunning false :!label _label))
    (Default|Run _playerchar _output_get))
  (:Completed
    (goto _label)))

(event Input|EnhancedActionEvents|EnhancedInputActionIA_Look
  (params (ActionValue :type Vector%202D%20Structure) (ElapsedSeconds :type Float%20%28double-precision%29) (TriggeredSeconds :type Float%20%28double-precision%29) (InputAction :type Input%20Action%20Object%20Reference :default "/Game/_GameManager/Inputs/InputActions/IA_Look.IA_Look"))
  (bind _camera_sensitivity (Variables|CameraSettings|GetCamera%20Sensitivity))
  (bind _campitchrange (Variables|CameraSettings|GetCamPitchRange))
  (bind _returnvalue (* ActionValue _camera_sensitivity))
  (bind (_x _y) (Math|Vector2D|BreakVector2D _returnvalue))
  ;[1 0.8688 0.3062] Look Around
  (bind _output_get (Variables|CameraSettings|SetCurrentCamRotation (Math|Rotator|MakeRotator 0.0 (Math|Float|Clamp(Float) (+ (* _y -1.0) (.Pitch (Math|Rotator|BreakRotator (Variables|CameraSettings|GetCurrentCamRotation)))) (.x _campitchrange) (.y _campitchrange)) (+ _x (.Yaw (Math|Rotator|BreakRotator (Variables|CameraSettings|GetCurrentCamRotation)))))))
  (bind _asbp_player_character (Utilities|Casting|CastToBP_PlayerCharacter (Game|GetPlayerCharacter 0)))
  (Transformation|SetWorldRotation (Variables|/Game/_GameManager/BP_PlayerCharacter.BP_PlayerCharacter_C|GetBoomStick _asbp_player_character) _output_get false false))

(event Input|EnhancedActionEvents|EnhancedInputActionIA_Sprint
  (params (ActionValue :type Boolean) (ElapsedSeconds :type Float%20%28double-precision%29) (TriggeredSeconds :type Float%20%28double-precision%29) (InputAction :type Input%20Action%20Object%20Reference :default "/Game/_GameManager/Inputs/InputActions/IA_Sprint.IA_Sprint"))
  ;[1 1 1] Running Behaviour
  (:Canceled
    (bind _output_get (Variables|Default|SetisRunning (not (Variables|Default|GetisRunning)) :!label _label))
    (Default|Run (Variables|Default|GetPlayerChar) _output_get))
  (:Completed
    (goto _label)))

(event Input|EnhancedActionEvents|EnhancedInputActionIA_Cast1
  (params (ActionValue :type Boolean) (ElapsedSeconds :type Float%20%28double-precision%29) (TriggeredSeconds :type Float%20%28double-precision%29) (InputAction :type Input%20Action%20Object%20Reference :default "/Game/_GameManager/Inputs/InputActions/IA_Cast1.IA_Cast1")))

(event EventBeginPlay
  ;[1 1 1] Set Mapping Context
  (Input|AddMappingContext (PlayerController|LocalPlayerSubsystems|GetEnhancedInputLocalPlayerSubsystem) "/Game/_GameManager/Inputs/IMC_Main.IMC_Main" 0 "(bIgnoreAllPressedKeysUntilRelease=True,bForceImmediately=False,bNotifyUserSettings=False)")
  (bind _asbp_player_character (Utilities|Casting|CastToBP_PlayerCharacter (Game|GetPlayerCharacter 0)))
  (Variables|Default|SetPlayerChar _asbp_player_character)
  (Variables|CameraSettings|SetCurrentCamRotation (Transformation|GetWorldRotation (Variables|/Game/_GameManager/BP_PlayerCharacter.BP_PlayerCharacter_C|GetBoomStick _asbp_player_character))))

(event EventTick
  (params (DeltaSeconds :type Float%20%28single-precision%29)))

(fn ConstructionScript)