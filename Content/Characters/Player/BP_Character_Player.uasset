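; Player character Blueprint that fires projectiles in the direction the camera faces.
; FireProjectile spawns a BP_Projectile at the mesh's Muzzle_01 socket with the camera's rotation, then sets its movement velocity along the camera's forward vector, scaled by ProjectileSpeed.
; CastProjectile is an empty event, and nothing in this Blueprint's graphs calls FireProjectile.
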(event Custom|FireProjectile
  (bind _camera (Variables|Default|GetCamera))
  (bind _returnvalue (Transformation|GetWorldRotation _camera))
  (bind _returnvalue_2 (Game|SpawnActorfromClass "/Game/Characters/BP_Projectile.BP_Projectile_C" (Math|Transform|MakeTransform (Transformation|GetSocketLocation (Variables|Character|GetMesh) "Muzzle_01") _returnvalue) "Undefined" "MultiplyWithRoot" 0 0))
  (Variables|/Script/Engine.MovementComponent|SetVelocity (Variables|/Game/Characters/BP_Projectile.BP_Projectile_C|GetProjectileMovement _returnvalue_2) (* (Math|Rotator|GetRotationXVector _returnvalue) (Variables|Default|GetProjectile%20Speed))))

(event Custom|Cast%20Projectile)

(event EventBeginPlay)

(event Collision|EventActorBeginOverlap
  (params (OtherActor :type Actor%20Object%20Reference)))

(event EventTick
  (params (DeltaSeconds :type Float%20%28single-precision%29)))

(fn ConstructionScript)